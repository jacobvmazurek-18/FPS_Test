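; FPSGameMode is a game mode that tracks how many drones remain in the level and shows the count on screen.
; On BeginPlay it creates a HUD widget, adds it to the viewport and sets the initial count from all DronePawn actors found.
; Its DroneDied function decrements that count and refreshes the HUD's drone text.
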(event EventBeginPlay
  ;[0.15 0.15 0.15 0.5] Add Game Mode HUD
  (bind _returnvalue (UserInterface|CreateWidget "/Game/Blueprints/HUD/GameModeHUD.GameModeHUD_C"))
  (bind _output_get (Variables|Default|SetGameModeHUD _returnvalue))
  (UserInterface|Viewport|AddtoViewport _output_get 0)
  ;[0.15 0.15 0.15 0.5] Set # of drones
  (bind _outactors (Actor|GetAllActorsOfClass "/Game/Blueprints/Drone/DronePawn.DronePawn_C"))
  (Variables|Default|SetNumberOfDrones (Utilities|Array|Length _outactors))
  (Rendering|Components|TextRender|SetText (Variables|/Game/Blueprints/HUD/GameModeHUD.GameModeHUD_C|GetDronesText (Variables|Default|GetGameModeHUD)) (Utilities|Text|ToText(Integer) (Utilities|Array|Length _outactors))))

(fn ConstructionScript)

(fn DroneDied
  (bind _result (Math|Integer|DecrementInt (Variables|Default|GetNumberOfDrones))
    (:%20%20
      (Rendering|Components|TextRender|SetText (Variables|/Game/Blueprints/HUD/GameModeHUD.GameModeHUD_C|GetDronesText (Variables|Default|GetGameModeHUD)) (Utilities|Text|ToText(Integer) _result)))))