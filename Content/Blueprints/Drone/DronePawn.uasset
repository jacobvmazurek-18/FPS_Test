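; Drone enemy pawn that patrols, chases the player and self-destructs on contact.
; Patrol uses AI MoveTo along linked PatrolPoints with a short pause, until the outer Overlap trigger switches GoalActor to the FPS_Character.
; Entering ExplodeSphere applies damage and calls Explode, as does running out of Health, playing sound and particles before destroying the drone.
; Tick sets an interpolated rotation targeting the current goal.
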(event OnComponentBeginOverlap(Overlap)
  (params (OverlappedComponent :type Primitive%20Component%20Object%20Reference) (OtherActor :type Actor%20Object%20Reference) (OtherComp :type Primitive%20Component%20Object%20Reference) (OtherBodyIndex :type Integer) (bFromSweep :type Boolean) (SweepResult :type Hit%20Result%20Structure%20%28by%20ref%29))
  ;[0.15 0.15 0.15 0.5] MoveTowardsPlayer
  (bind _asfps_character (Utilities|Casting|CastToFPS_Character OtherActor))
  (CallFunction|MovetoGoalTarget _asfps_character))

(event OnComponentBeginOverlap(ExplodeSphere)
  (params (OverlappedComponent :type Primitive%20Component%20Object%20Reference) (OtherActor :type Actor%20Object%20Reference) (OtherComp :type Primitive%20Component%20Object%20Reference) (OtherBodyIndex :type Integer) (bFromSweep :type Boolean) (SweepResult :type Hit%20Result%20Structure%20%28by%20ref%29))
  ;[0.15 0.15 0.15 0.5] Explode
  (Utilities|Casting|CastToFPS_Character OtherActor)
  (Game|Damage|ApplyDamage 0 (Variables|Default|GetDamage) 0 0)
  (CallFunction|Explode))

(event Custom|OnTakeAnyDamage_Event
  (params (DamagedActor :type Actor%20Object%20Reference) (Damage :type Float%20%28single-precision%29) (DamageType :type Damage%20Type%20Object%20Reference) (InstigatedBy :type Controller%20Object%20Reference) (DamageCauser :type Actor%20Object%20Reference))
  ;[0.15 0.15 0.15 0.5] TakingDamage
  (bind _output_get (Variables|Default|SetHealth (- (Variables|Default|GetHealth) Damage)))
  (if (<= _output_get 0.0)
    (CallFunction|Explode)))

(event Custom|MoveToGoalTarget
  (params (New%20Goal%20Target :type Actor%20Object%20Reference))
  ;[0.15 0.15 0.15 0.5] ?
  (bind _output_get (Variables|Default|SetGoalActor New%20Goal%20Target))
  (AI|AIMoveTo self "0, 0, 0" _output_get 25.0 false))

(event EventTick
  (params (DeltaSeconds :type Float%20%28single-precision%29))
  (bind _goalactor (Variables|Default|GetGoalActor))
  ;[0.15 0.15 0.15 0.5] Rotation
  (Utilities|IsValid _goalactor
    (:Is%20Valid
      (Transformation|SetActorRotation (Math|Interpolation|RInterpTo (Math|Conversions|RotationFromXVector (Transformation|GetActorLocation)) (Math|Rotator|FindLookatRotation (Transformation|GetActorLocation) (Transformation|GetActorLocation _goalactor)) 0.0 0.0)))))

(event EventBeginPlay
  ;[0.15 0.15 0.15 0.5] TakingDamage
  (EventDispatchers|AssignOnTakeAnyDamage (delegate Custom|OnTakeAnyDamage_Event))
  (Utilities|Patrol))

(fn ConstructionScript)

(fn Explode
  (Audio|PlaySoundatLocation "/Game/StarterContent/Audio/Explosion_Cue.Explosion_Cue" (Transformation|GetActorLocation) "0, 0, 0" 1.0 1.0 0.0 0 0 0 0)
  (Effects|SpawnEmitteratLocation "/Game/StarterContent/Particles/P_Explosion.P_Explosion" (Transformation|GetActorLocation))
  (Actor|DestroyActor))